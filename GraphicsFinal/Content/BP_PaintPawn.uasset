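; BP_PaintPawn is a mouse-driven brush pawn that paints on and erases from a BP_Plane found in the level at BeginPlay.
; Each tick it traces under the cursor, storing the hit position and its movement since the last hit as mouse velocity, and moves a Sphere marker there.
; Holding left mouse calls the plane's Draw with position, intensity-scaled velocity and brush size; holding right mouse calls Erase at that position.
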(event EventBeginPlay
  (Variables|/Script/Engine.PlayerController|SetbShowMouseCursor (Game|GetPlayerController 0) true)
  (bind _outactors (Actor|GetAllActorsOfClass "/Game/BP_Plane.BP_Plane_C"))
  (Variables|Default|SetPlane (Utilities|Array|Get(acopy) _outactors)))

(event EventTick
  (params (DeltaSeconds :type Float%20%28single-precision%29))
  (CallFunction|TraceUnderMouse)
  (CallFunction|UpdateSphereLoc)
  (Utilities|FlowControl|Sequence
    (:then_0
      (if (Variables|Default|GetisLeftMouseDown)
        (bind _output_get (Variables|Default|SetVelocity (* (Variables|Default|GetMouseVelocity) (Variables|Default|GetIntensity))))
        (Default|Draw (Variables|Default|GetPlane) (Variables|Default|GetPosition) _output_get (Variables|Default|GetBrushSize))))
    (:then_1
      (if (Variables|Default|GetisRightMouseDown)
        (Default|Erase (Variables|Default|GetPlane) (Variables|Default|GetPosition))))))

(event Input|MouseEvents|LeftMouseButton
  (params (Key :type Key%20Structure :default "None"))
  (:Pressed
    (Variables|Default|SetisLeftMouseDown true))
  (:Released
    (Variables|Default|SetisLeftMouseDown false)))

(event Input|MouseEvents|RightMouseButton
  (params (Key :type Key%20Structure :default "None"))
  (:Pressed
    (Variables|Default|SetisRightMouseDown true))
  (:Released
    (Variables|Default|SetisRightMouseDown false)))

(fn ConstructionScript)

(fn TraceUnderMouse
  (bind _returnvalue (Game|GetPlayerController 0))
  (bind (_hitresult _returnvalue_2) (Game|Player|GetHitResultUnderCursorbyChannel _returnvalue "TraceTypeQuery1" true))
  (if _returnvalue_2
    (Variables|Default|SetMouseVelocity (- (.location _hitresult) (Variables|Default|GetPosition)))
    (Variables|Default|SetPosition (.location _hitresult))
    (return)))

(fn UpdateSphereLoc
  (Transformation|SetWorldLocation (Variables|Default|GetSphere) (Variables|Default|GetPosition) false false))